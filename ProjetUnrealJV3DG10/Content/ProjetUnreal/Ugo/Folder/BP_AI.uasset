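; AI character that moves toward the player at a speed driven by a recurring sound, in a red-light/green-light style.
; BeginPlay starts AIMoveTo on the player controller, binds to the first-person character's movement event and launches EmitSound.
; EmitSound loops on random delays, setting crouch speed during playback and zero speed afterward.
; SetSpeedRelativeToPlayer, apparently the bound callback, switches to run speed while the sound plays.
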(event Custom|EmitSound
  (bind _sound (Variables|Default|GetSound))
  (Utilities|FlowControl|Delay (Math|Random|RandomFloatinRange (Variables|Default|GetMinSoundDelay) (Variables|Default|GetMaxSoundDelay)))
  (Audio|PlaySoundatLocation _sound (Transformation|GetActorLocation) "0, 0, 0" 1.0 1.0 0.0 0 0 0 0)
  (Variables|Default|SetIsPlayingSound true)
  (Variables|/Script/Engine.CharacterMovementComponent|SetMaxWalkSpeed (Variables|Character|GetCharacterMovement) (Variables|Default|GetCrouchSpeed))
  (Utilities|FlowControl|Delay (Variables|/Script/Engine.SoundBase|GetDuration _sound))
  (Variables|Default|SetIsPlayingSound false)
  (Variables|/Script/Engine.CharacterMovementComponent|SetMaxWalkSpeed (Variables|Character|GetCharacterMovement) 0.0)
  (CallFunction|EmitSound))

(event Custom|SetSpeedRelativeToPlayer
  (if (Variables|Default|GetIsPlayingSound)
    (Variables|/Script/Engine.CharacterMovementComponent|SetMaxWalkSpeed (Variables|Character|GetCharacterMovement) (Variables|Default|GetRunSpeed))))

(event EventBeginPlay
  (bind _returnvalue (Actor|GetActorOfClass "/Game/FirstPerson/Blueprints/BP_FirstPersonCharacter.BP_FirstPersonCharacter_C"))
  (bind _output_get (Variables|Default|SetPlayer _returnvalue))
  (EventDispatchers|BindEventtoPlayerMoving _output_get (EventDispatchers|CreateEvent :!event Custom|SetSpeedRelativeToPlayer))
  (Variables|/Script/Engine.CharacterMovementComponent|SetMaxWalkSpeed (Variables|Character|GetCharacterMovement) (Variables|Default|GetWalkSpeed))
  (AI|AIMoveTo self "0, 0, 0" (Game|GetPlayerController 0) 5.0 false
    (:then
      (CallFunction|EmitSound))))

(fn ConstructionScript)