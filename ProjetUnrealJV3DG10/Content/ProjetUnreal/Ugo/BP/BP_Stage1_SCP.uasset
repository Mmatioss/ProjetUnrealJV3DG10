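; BP_Stage1_SCP is a first-stage SCP enemy that turns into a BP_AI when interacted with.
; On start it registers with GI_Jam and applies a VHS post-process; its audio trigger plays a sound and saves the player's restart transform.
; Interact freezes the player, adds light flickering, spawns the AI and calls ShowFlesh.
; After a delay it restores view and movement, spawns an explosion at the player and destroys itself.
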(event OnComponentBeginOverlap(AudioTrigger)
  (params (OverlappedComponent :type Primitive%20Component%20Object%20Reference) (OtherActor :type Actor%20Object%20Reference) (OtherComp :type Primitive%20Component%20Object%20Reference) (OtherBodyIndex :type Integer) (bFromSweep :type Boolean) (SweepResult :type Hit%20Result%20Structure%20%28by%20ref%29))
  (bind _as_gi_jam (Variables|Default|GetAs%20GI%20Jam))
  (Utilities|Casting|CastToBP_FirstPersonCharacter OtherActor)
  (Variables|/Game/ProjetUnreal/Ugo/BP/GI_Jam.GI_Jam_C|SetPlayerRestartPosition _as_gi_jam (Transformation|GetActorTransform OtherActor))
  (Variables|/Game/ProjetUnreal/Ugo/BP/GI_Jam.GI_Jam_C|SetEnemyLocation _as_gi_jam (Transformation|GetActorTransform))
  (Audio|PlaySoundatLocation (Variables|Default|GetSoundToPlay) (Transformation|GetActorLocation) "0, 0, 0" 1.0 1.0 0.0 0 0 0 0))

(event EventBeginPlay
  (Components|Sphere|SetSphereRadius (Variables|Default|GetAudioTrigger) (Variables|Default|GetAudioTriggerScale) true)
  (bind _returnvalue (Actor|GetActorOfClass "/Script/Engine.PostProcessVolume"))
  (Variables|Default|SetPostProcess _returnvalue)
  (bind _returnvalue_2 (Actor|GetActorOfClass "/Game/FirstPerson/Blueprints/BP_FirstPersonCharacter.BP_FirstPersonCharacter_C"))
  (Variables|Default|SetPlayer _returnvalue_2)
  (bind _asgi_jam (Utilities|Casting|CastToGI_Jam (Game|GetGameInstance)))
  (bind _output_get (Variables|Default|SetAs%20GI%20Jam _asgi_jam))
  (Variables|/Game/ProjetUnreal/Ugo/BP/GI_Jam.GI_Jam_C|SetEnemyLocation _output_get (Transformation|GetActorTransform))
  (Variables|/Game/ProjetUnreal/Ugo/BP/GI_Jam.GI_Jam_C|SetEnemy _output_get self)
  (bind _returnvalue_3 (Rendering|Material|CreateDynamicMaterialInstance "/Game/ProjetUnreal/Materials/PostProcess/MI_VHS.MI_VHS" "None" "None" :!class /Script/Engine.KismetMaterialLibrary))
  (Variables|/Script/Engine.PostProcessVolume|SetSettings (Variables|Default|GetPostProcess) (Utilities|Struct|MakePostProcessSettings 0.0 0.0 0.0 (Utilities|Struct|MakeWeightedBlendables (Utilities|Array|MakeArray (Utilities|Struct|MakeWeightedBlendable 1.0 _returnvalue_3))))))

(event EventInteract
  (bind _returnvalue (Transformation|GetActorTransform))
  (Pawn|Components|CharacterMovement|DisableMovement (Variables|/Script/Engine.Character|GetCharacterMovement (Variables|Default|GetPlayer)))
  (bind _returnvalue_2 (Rendering|Material|CreateDynamicMaterialInstance "/Game/ProjetUnreal/Ugo/Materials/M_LightFlickering.M_LightFlickering" "None" "None" :!class /Script/Engine.KismetMaterialLibrary))
  (bind _returnvalue_3 (Rendering|Material|CreateDynamicMaterialInstance "/Game/ProjetUnreal/Materials/PostProcess/MI_VHS.MI_VHS" "None" "None" :!class /Script/Engine.KismetMaterialLibrary))
  (Variables|/Script/Engine.PostProcessVolume|SetSettings (Variables|Default|GetPostProcess) (Utilities|Struct|MakePostProcessSettings 0.0 0.0 0.0 (Utilities|Struct|MakeWeightedBlendables (Utilities|Array|MakeArray (Utilities|Struct|MakeWeightedBlendable 1.0 _returnvalue_2) (Utilities|Struct|MakeWeightedBlendable 1.0 _returnvalue_3)))))
  (Utilities|FlowControl|Delay 0.2)
  (Game|SpawnActorfromClass "/Game/ProjetUnreal/Ugo/BP/BP_AI.BP_AI_C" (Math|Transform|MakeTransform (Math|Vector|MakeVector (.x (.location _returnvalue)) (.y (.location _returnvalue)) (+ (.z (.location _returnvalue)) 1e+02)) (.rotation _returnvalue) (.scale _returnvalue)) "AlwaysSpawn" "MultiplyWithRoot" 0 0)
  (Default|ShowFlesh (Variables|Default|GetAs%20GI%20Jam))
  (Utilities|FlowControl|Delay 2.0)
  (bind _returnvalue_4 (Rendering|Material|CreateDynamicMaterialInstance "/Game/ProjetUnreal/Materials/PostProcess/MI_VHS.MI_VHS" "None" "None" :!class /Script/Engine.KismetMaterialLibrary))
  (Variables|/Script/Engine.PostProcessVolume|SetSettings (Variables|Default|GetPostProcess) (Utilities|Struct|MakePostProcessSettings 0.0 0.0 0.0 (Utilities|Struct|MakeWeightedBlendables (Utilities|Array|MakeArray (Utilities|Struct|MakeWeightedBlendable 1.0 _returnvalue_4)))))
  (Pawn|Components|CharacterMovement|SetMovementMode (Variables|/Script/Engine.Character|GetCharacterMovement (Variables|Default|GetPlayer)) "MOVE_Walking" 0)
  (Effects|SpawnEmitteratLocation "/Game/StarterContent/Particles/P_Explosion.P_Explosion" (Transformation|GetActorLocation (Game|Player|GetPlayerPawn 0)) "0, 0, 0" "5.000000,5.000000,5.000000" false)
  (Actor|DestroyActor))

(fn ConstructionScript)