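; Enemy AI that chases the first-person player and triggers a jumpscare on reaching them.
; A looping timer drives the chase, while a self-recalling event plays sounds at random intervals.
; Tick sets speed: walk normally, crouch speed during sound, run if the player moves during it, tracked through player movement bindings.
; On contact it shows the screamer, teleports the player to restart, spawns a BP_Stage1_SCP and destroys itself.
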(event Custom|EmitSound
  (bind _sound (Variables|Default|GetSound))
  (Utilities|FlowControl|Delay (Math|Random|RandomFloatinRange (Variables|Default|GetMinSoundDelay) (Variables|Default|GetMaxSoundDelay)))
  (Audio|PlaySoundatLocation _sound (Transformation|GetActorLocation) "0, 0, 0" 1.0 1.0 0.0 0 0 0 0)
  (Variables|Default|SetIsPlayingSound true)
  (Variables|/Script/Engine.CharacterMovementComponent|SetMaxWalkSpeed (Variables|Character|GetCharacterMovement) (Variables|Default|GetCrouchSpeed))
  (Utilities|FlowControl|Delay (Variables|/Script/Engine.SoundBase|GetDuration _sound))
  (Variables|Default|SetIsPlayingSound false)
  (Variables|/Script/Engine.CharacterMovementComponent|SetMaxWalkSpeed (Variables|Character|GetCharacterMovement) (Variables|Default|GetWalkSpeed))
  (CallFunction|EmitSound))

(event Custom|OnPlayerMoving
  (Variables|Default|SetIsPlayerMoving true))

(event Custom|OnPlayerStoppedMoving
  (Variables|Default|SetIsPlayerMoving false))

(event Custom|MoveToPlayer
  (bind _player (Variables|Default|GetPlayer))
  (bind _player_2 (Variables|Default|GetPlayer))
  (AI|AIMoveTo self (Transformation|GetActorLocation _player_2) _player_2 5.0 false
    (:then
      (CallFunction|EmitSound))
    (:OnSuccess
      (Pawn|Components|CharacterMovement|SetMovementMode (Variables|Character|GetCharacterMovement) "MOVE_None" 0)
      (bind _returnvalue (UserInterface|CreateWidget "/Game/ProjetUnreal/Ugo/BP/WBP_Screamer.WBP_Screamer_C"))
      (Audio|PlaySound2D (Variables|Default|GetScreamerSound) 1.0 1.0 0.0 0 0)
      (Utilities|FlowControl|Delay 0.2)
      (UserInterface|Viewport|AddtoViewport _returnvalue 0)
      (Transformation|SetActorTransform _player (Variables|/Game/ProjetUnreal/Ugo/BP/GI_Jam.GI_Jam_C|GetPlayerRestartPosition (Variables|Default|GetAs%20GI%20Jam)) false true)
      (Pawn|Components|CharacterMovement|SetMovementMode (Variables|/Script/Engine.Character|GetCharacterMovement _player) "MOVE_None" 0)
      (Game|SpawnActorfromClass "/Game/ProjetUnreal/Ugo/BP/BP_Stage1_SCP.BP_Stage1_SCP_C" (Variables|/Game/ProjetUnreal/Ugo/BP/GI_Jam.GI_Jam_C|GetEnemyLocation (Variables|Default|GetAs%20GI%20Jam)) "AdjustIfPossibleButAlwaysSpawn" "MultiplyWithRoot" 0 0)
      (Utilities|FlowControl|Delay (Variables|/Script/Engine.SoundBase|GetDuration (Variables|Default|GetScreamerSound)))
      (Widget|RemovefromParent _returnvalue)
      (Pawn|Components|CharacterMovement|SetMovementMode (Variables|/Script/Engine.Character|GetCharacterMovement (Variables|Default|GetPlayer)) "MOVE_Walking" 0)
      (Actor|DestroyActor))))

(event EventTick
  (params (DeltaSeconds :type Float%20%28single-precision%29))
  (bind _isplayingsound (Variables|Default|GetIsPlayingSound))
  (bind _charactermovement (Variables|Character|GetCharacterMovement))
  (if (and _isplayingsound (Variables|Default|GetIsPlayerMoving))
    (Variables|/Script/Engine.CharacterMovementComponent|SetMaxWalkSpeed (Variables|Character|GetCharacterMovement) (Variables|Default|GetRunSpeed))
    (elif _isplayingsound
      (Variables|/Script/Engine.CharacterMovementComponent|SetMaxWalkSpeed _charactermovement (Variables|Default|GetCrouchSpeed))
      (else
        (Variables|/Script/Engine.CharacterMovementComponent|SetMaxWalkSpeed _charactermovement (Variables|Default|GetWalkSpeed))))))

(event EventBeginPlay
  (bind _asgi_jam (Utilities|Casting|CastToGI_Jam (Game|GetGameInstance)))
  (Variables|Default|SetAs%20GI%20Jam _asgi_jam)
  (bind _returnvalue (Actor|GetActorOfClass "/Game/FirstPerson/Blueprints/BP_FirstPersonCharacter.BP_FirstPersonCharacter_C"))
  (Variables|Default|SetPlayer _returnvalue)
  (Variables|/Script/Engine.CharacterMovementComponent|SetMaxWalkSpeed (Variables|Character|GetCharacterMovement) 0.0)
  (Utilities|FlowControl|Delay 1.5)
  (Variables|/Script/Engine.CharacterMovementComponent|SetMaxWalkSpeed (Variables|Character|GetCharacterMovement) (Variables|Default|GetWalkSpeed))
  (Utilities|Time|SetTimerbyEvent (EventDispatchers|CreateEvent :!event Custom|MoveToPlayer) 2.0 true)
  (EventDispatchers|BindEventtoPlayerMoving (Variables|Default|GetPlayer) (EventDispatchers|CreateEvent :!event Custom|OnPlayerMoving))
  (EventDispatchers|BindEventtoPlayerStoppedMoving (Variables|Default|GetPlayer) (EventDispatchers|CreateEvent :!event Custom|OnPlayerStoppedMoving)))

(fn ConstructionScript)