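; BP_AudioManager handles background music and Dr. Clef's voice lines with their subtitles.
; On BeginPlay outside the main menu, it gets the subtitle widget from the first-person character, then after a delay plays the intro line and subtitle.
; A mid-game event chains two more lines with a timed delay.
; Music events stop playback or choose one of three tracks by index on a separate audio component.
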(event Custom|PlayAudioTalkStart
  (bind _audiotalk (Variables|Default|GetAudioTalk))
  ;[0.15 0.15 0.15 0.5] playAudioTalk
  (Audio|Components|Audio|SetSound _audiotalk "/Game/ProjetUnreal/Audio/Talk/Dr_clef_line_intro.Dr_clef_line_intro")
  (Audio|Components|Audio|Play _audiotalk 0.0))

(event Custom|PlayBackGroundMusic
  (bind _audiomusic (Variables|Default|GetAudioMusic))
  ;[0.15 0.15 0.15 0.5] PlayBackGroundMusic
  (switch int (Variables|Default|GetNbBackGroundMusic)
    (:0
      (Audio|Components|Audio|SetSound _audiomusic "/Game/ProjetUnreal/Audio/Music/OST_filled_lungs.OST_filled_lungs")
      (Audio|Components|Audio|Play _audiomusic 0.0))
    (:1
      (Audio|Components|Audio|SetSound _audiomusic "/Game/ProjetUnreal/Audio/Music/OST_2_Not_so_foreboding_entrance.OST_2_Not_so_foreboding_entrance")
      (Audio|Components|Audio|Play _audiomusic 0.0))
    (:2
      (Audio|Components|Audio|SetSound _audiomusic "/Game/ProjetUnreal/Audio/Music/OST_3_In_the_meat_of_it_loop.OST_3_In_the_meat_of_it_loop")
      (Audio|Components|Audio|Play _audiomusic 0.0))))

(event Custom|StopBackGroundMusic
  ;[0.15 0.15 0.15 0.5] StopBackGroundMusic
  (Audio|Components|Audio|Stop (Variables|Default|GetAudioMusic)))

(event Custom|PlayAudioTalkMid
  (bind _audiotalk (Variables|Default|GetAudioTalk))
  (bind _audiotalk_2 (Variables|Default|GetAudioTalk))
  ;[0.15 0.15 0.15 0.5] playAudioTalk
  (Default|Talk2 (Variables|Default|GetSubtitle%20Widget))
  (Audio|Components|Audio|SetSound _audiotalk_2 "/Game/ProjetUnreal/Audio/Talk/Dr_clef_line_2.Dr_clef_line_2")
  (Audio|Components|Audio|Play _audiotalk_2 0.0)
  (Utilities|FlowControl|Delay 23.0)
  (Audio|Components|Audio|SetSound _audiotalk "/Game/ProjetUnreal/Audio/Talk/Dr_clef_line_3.Dr_clef_line_3")
  (Audio|Components|Audio|Play _audiotalk 0.0))

(event EventBeginPlay
  ;[0.15 0.15 0.15 0.5] BeginPlay
  (bind _returnvalue (Game|GetCurrentLevelName true))
  (if (not (Utilities|Enum|Equal(Enum) "L_MainMenu" _returnvalue))
    (Utilities|FlowControl|Delay 0.5)
    (bind _asbp_first_person_character (Utilities|Casting|CastToBP_FirstPersonCharacter (Game|Player|GetPlayerPawn 0)))
    (bind _output_get (Variables|Default|SetSubtitle%20Widget (Variables|/Game/FirstPerson/Blueprints/BP_FirstPersonCharacter.BP_FirstPersonCharacter_C|GetSubtitleWidget _asbp_first_person_character)))
    (Utilities|FlowControl|Delay 4.0)
    (CallFunction|PlayAudioTalkStart)
    (Default|Talk1 _output_get)))

(fn ConstructionScript)