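; BP_RandomEvent plays random sounds at the player pawn's location on a repeating, randomly timed loop.
; StartLoop sets IsPlaying and calls StartRandomSound, which waits between MinTimeRandom and MaxTimeRandom, plays a SoundList entry, then calls itself again.
; EndRandomSound clears IsPlaying, but the loop's branch is hardwired true, so the loop keeps running.
; The random index range includes SoundList's length, one past the last element.
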(event Custom|StartRandomSound
  (bind _soundlist (Variables|Default|GetSoundList))
  ;[0.15 0.15 0.15 0.5] Start random sound
  (if true
    (Utilities|FlowControl|Delay (Math|Random|RandomFloatinRange (Variables|Default|GetMinTimeRandom) (Variables|Default|GetMaxTimeRandom)))
    (Audio|PlaySoundatLocation (Utilities|Array|Get(acopy) _soundlist (Math|Conversions|ToInteger(Byte) (Class|KismetMathLibrary|RandomInteger64inRange 0 (Class|KismetMathLibrary|ToInt64(Integer) (Utilities|Array|Length _soundlist))))) (Transformation|GetActorLocation (Game|Player|GetPlayerPawn 0)) "0, 0, 0" 1.0 1.0 0.0 0 0 0 0)
    (CallFunction|StartRandomSound)))

(event Custom|EndRandomSound
  ;[0.15 0.15 0.15 0.5] Disable random sound
  (Variables|Default|SetIsPlaying false))

(event Custom|StartLoop
  ;[0.15 0.15 0.15 0.5] Start loop
  (Variables|Default|SetIsPlaying true)
  (CallFunction|StartRandomSound))

(fn ConstructionScript)