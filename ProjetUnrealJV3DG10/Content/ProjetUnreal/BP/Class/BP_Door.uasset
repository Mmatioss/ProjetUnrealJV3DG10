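; BP_Door is a two-panel sliding door for level start or end, set by IsEnd, that opens or attempts closing at BeginPlay.
; An overlapping first-person character that has touched the SCP triggers closing; end doors also show the win widget and pause the game.
; Separate timelines lerp panels from their current positions along right vectors, guarded by IsOpen.
; The close path uses the open path's offsets and also sets IsOpen true.
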(event OnComponentBeginOverlap(EnterCollision)
  (params (OverlappedComponent :type Primitive%20Component%20Object%20Reference) (OtherActor :type Actor%20Object%20Reference) (OtherComp :type Primitive%20Component%20Object%20Reference) (OtherBodyIndex :type Integer) (bFromSweep :type Boolean) (SweepResult :type Hit%20Result%20Structure%20%28by%20ref%29))
  ;[0.15 0.15 0.15 0.5] Enter/Exit Collision
  (bind _asbp_first_person_character (Utilities|Casting|CastToBP_FirstPersonCharacter OtherActor))
  (if (Variables|/Game/FirstPerson/Blueprints/BP_FirstPersonCharacter.BP_FirstPersonCharacter_C|GetHasTouchedSCP _asbp_first_person_character)
    (CallFunction|PlayCloseAnim)
    (if (Variables|Default|GetIsEnd)
      (bind _returnvalue (UserInterface|CreateWidget "/Game/ProjetUnreal/UI/WBP_Win.WBP_Win_C" (Game|GetPlayerController 0)))
      (UserInterface|Viewport|AddtoViewport _returnvalue 0)
      (Game|SetGamePaused true))))

(event Custom|PlayOpenAnim
  (bind _door2 (Variables|Default|Getdoor2))
  (bind _door1 (Variables|Default|Getdoor1))
  (bind _relativelocation (Variables|/Script/Engine.SceneComponent|GetRelativeLocation _door1))
  (bind _relativelocation_2 (Variables|/Script/Engine.SceneComponent|GetRelativeLocation _door2))
  ;[0.15 0.15 0.15 0.5] PlayOpenAnim
  (Variables|Default|SetInAnim true)
  (if (not (Variables|Default|GetIsOpen))
    (Variables|Default|SetIsOpen true)
    (bind _alpha (Timeline|TimeLineOpenDoor PlayFromStart)
      (:Update
        (Transformation|SetRelativeLocation _door1 (Math|Vector|Lerp(Vector) _relativelocation (+ _relativelocation (* (Math|Vector|GetRightVector _door1) (* (Variables|Default|GetDistanceMoveDoor) -1.0))) _alpha) false false)
        (Transformation|SetRelativeLocation _door2 (Math|Vector|Lerp(Vector) _relativelocation_2 (+ _relativelocation_2 (* (Math|Vector|GetRightVector _door2) (* (Variables|Default|GetDistanceMoveDoor) 1.0))) _alpha) false false))
      (:Finished
        (Variables|Default|SetInAnim false)))))

(event Custom|PlayCloseAnim
  (bind _door2 (Variables|Default|Getdoor2))
  (bind _door1 (Variables|Default|Getdoor1))
  (bind _relativelocation (Variables|/Script/Engine.SceneComponent|GetRelativeLocation _door1))
  (bind _relativelocation_2 (Variables|/Script/Engine.SceneComponent|GetRelativeLocation _door2))
  ;[0.15 0.15 0.15 0.5] PlayCloseAnim
  (Variables|Default|SetInAnim true)
  (if (Variables|Default|GetIsOpen)
    (Variables|Default|SetIsOpen true)
    (bind _alpha (Timeline|Timeline PlayFromStart)
      (:Update
        (Transformation|SetRelativeLocation _door2 (Math|Vector|Lerp(Vector) _relativelocation_2 (+ _relativelocation_2 (* (Math|Vector|GetRightVector _door2) (* (Variables|Default|GetDistanceMoveDoor) 1.0))) _alpha) false false)
        (Transformation|SetRelativeLocation _door1 (Math|Vector|Lerp(Vector) _relativelocation (+ _relativelocation (* (Math|Vector|GetRightVector _door1) (* (Variables|Default|GetDistanceMoveDoor) -1.0))) _alpha) false false))
      (:Finished
        (Variables|Default|SetInAnim false)))))

(event EventBeginPlay
  ;[0.15 0.15 0.15 0.5] BeginPlay
  (if (not (Variables|Default|GetIsEnd))
    (CallFunction|PlayOpenAnim)
    (else
      (CallFunction|PlayCloseAnim))))

(fn ConstructionScript)